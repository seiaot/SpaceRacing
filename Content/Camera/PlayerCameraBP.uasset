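; Player camera actor that hands its spring arm and camera to the player and becomes the active view.
; On BeginPlay it gets the player through MyGameInstance and calls ChangeCamera with MPSpringArm and MPCamera, then sets itself as player controller 0's view target.
; It stops before both steps if the game instance cast fails, and has no active tick or overlap logic.
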(event `self.ReceiveBeginPlay`
  (`parent.ReceiveBeginPlay`)
  (bind _asmy_game_instance (cast `MyGameInstance` (`GameplayStatics.GetGameInstance`)))
  (`PlayerChara.ChangeCamera` (`MyGameInstance.GetPlayer` _asmy_game_instance) (`self.m_pSpringArm`) (`self.m_pCamera`))
  (`PlayerController.SetViewTargetWithBlend` (`GameplayStatics.GetPlayerController` 0) self 0.0 "VTBlend_Linear" 0.0 false))

(fn `UserConstructionScript`
  (`parent.UserConstructionScript`))