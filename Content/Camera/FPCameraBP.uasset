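; First-person camera actor, going by its name, that follows the player's position and orientation.
; On BeginPlay it casts the game instance to MyGameInstance and caches the player reference from it.
; Each Tick it copies the player's actor location and rotation onto itself directly, with no offset or smoothing.
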(event `self.ReceiveBeginPlay`
  (`parent.ReceiveBeginPlay`)
  (bind _asmy_game_instance (cast `MyGameInstance` (`GameplayStatics.GetGameInstance`)))
  (set `self.Player` (`MyGameInstance.GetPlayer` _asmy_game_instance)))

(event `self.ReceiveTick`
  (params (DeltaSeconds :type "Float (single-precision)"))
  (bind (_returnvalue_location _returnvalue_rotation) (`KismetMathLibrary.BreakTransform` (`self.GetTransform` (`self.Player`))))
  (`parent.ReceiveTick` DeltaSeconds)
  (`self.K2_SetActorLocationAndRotation` _returnvalue_location _returnvalue_rotation))

(fn `UserConstructionScript`
  (`parent.UserConstructionScript`))